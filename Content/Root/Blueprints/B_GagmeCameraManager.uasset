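; B_GagmeCameraManager is a camera manager Blueprint with an unfinished or disabled top-down follow camera.
; BlueprintUpdateCamera has an empty live body, as its camera logic is disconnected and never runs.
; That logic targets a point above the camera target through CalculateTarget, snaps there the first time, then eases with VInterpTo under a fixed downward rotation and FOV.
; The event graph and construction script are empty.
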(fn `BlueprintUpdateCamera`
  (params (CameraTarget :type "Actor Object Reference"))
  (returns (NewCameraLocation :type "Vector Structure") (NewCameraRotation :type "Rotator Structure") (NewCameraFOV :type "Float (single-precision)") (ReturnValue :type Boolean))
  (locals (`-Target` :type "Vector Structure" :default (0.0 0.0 0.0))))

(fn `CalculateTarget`
  (params (A :type "Vector Structure"))
  (returns (ReturnValue :type "Vector Structure"))
  (return (+ A (* (0.0 0.0 1.0) 700.0))))

(fn `UserConstructionScript`)