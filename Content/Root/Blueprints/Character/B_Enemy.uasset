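; B_Enemy is an enemy that patrols along a spline and catches the player's ghost pawn.
; Each tick advances distance by MoveSpeed and places Boy2Anim at that spline transform with a yaw offset, restarting past the end if Loop is set.
; Overlapping the caught sphere calls Caught on B_GhostPawn.
; The sense sphere only casts, and state-based movement logic is left disconnected.
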(event `self.ReceiveBeginPlay`)

(event `self.ReceiveTick`
  (params (DeltaSeconds :type "Float (single-precision)"))
  (bind _returnvalue (`SplineComponent.GetTransformAtDistanceAlongSpline` (`self.Spline`) (`self.Current Distance`) "Local" false))
  (set `self.Current Distance` (+ (* DeltaSeconds (`self.Move Speed`)) (`self.Current Distance`)))
  (`SceneComponent.K2_SetRelativeTransform` (`self.Boy_2Anim`) (`KismetMathLibrary.MakeTransform` (`KismetMathLibrary.MakeVector` (.x (.location _returnvalue)) (.y (.location _returnvalue)) (.z (.location _returnvalue))) (`KismetMathLibrary.MakeRotator` (.roll (.rotation _returnvalue)) (.pitch (.rotation _returnvalue)) (- (.yaw (.rotation _returnvalue)) 90.0)) (`SceneComponent.RelativeScale3D` (`self.Boy_2Anim`))) false false)
  (if (`self.Loop`)
    (if (> (`self.Current Distance`) (`SplineComponent.GetSplineLength` (`self.Spline`)))
      (set `self.Current Distance` 0.0))))

(event `CustomEvent`)

(event `self.Detection CAUGHT Sphere.OnComponentBeginOverlap`
  (params (OverlappedComponent :type "PrimitiveComponent Object Reference") (OtherActor :type "Actor Object Reference") (OtherComp :type "PrimitiveComponent Object Reference") (OtherBodyIndex :type Integer) (bFromSweep :type Boolean) (SweepResult :type "HitResult Structure (by ref)"))
  (bind _asb_ghost_pawn (cast `/Game/Root/Blueprints/Character/B_GhostPawn` OtherActor))
  (`/Game/Root/Blueprints/Character/B_GhostPawn.Caught` _asb_ghost_pawn))

(event `self.Detection SENSE sphere.OnComponentBeginOverlap`
  (params (OverlappedComponent :type "PrimitiveComponent Object Reference") (OtherActor :type "Actor Object Reference") (OtherComp :type "PrimitiveComponent Object Reference") (OtherBodyIndex :type Integer) (bFromSweep :type Boolean) (SweepResult :type "HitResult Structure (by ref)"))
  (cast `/Game/Root/Blueprints/Character/B_GhostPawn` OtherActor))

(fn `UserConstructionScript`)