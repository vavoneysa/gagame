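; Standing AI enemy that catches the player's ghost pawn when it enters the enemy's catch sphere.
; On overlap it plays a one-shot animation on the ghost's THEGhostTest2 component, waits briefly, then calls Caught on that pawn.
; Spline movement, the seeing flag and blackboard updates are disconnected leftovers that never run, and BeginPlay and Tick are empty.
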(event `self.ReceiveBeginPlay`)

(event `self.ReceiveTick`
  (params (DeltaSeconds :type "Float (single-precision)")))

(event `self.CaughtSphere.OnComponentBeginOverlap`
  (params (OverlappedComponent :type "PrimitiveComponent Object Reference") (OtherActor :type "Actor Object Reference") (OtherComp :type "PrimitiveComponent Object Reference") (OtherBodyIndex :type Integer) (bFromSweep :type Boolean) (SweepResult :type "HitResult Structure (by ref)"))
  (bind _asb_ghost_pawn (cast `/Game/Root/Blueprints/Character/B_GhostPawn` OtherActor))
  (`SkeletalMeshComponent.PlayAnimation` (`/Game/Root/Blueprints/Character/B_GhostPawn.THEGhost_test2` _asb_ghost_pawn) null false)
  (`KismetSystemLibrary.Delay` 2.0)
  (`/Game/Root/Blueprints/Character/B_GhostPawn.Caught` _asb_ghost_pawn))

(fn `UserConstructionScript`)