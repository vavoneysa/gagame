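; Ghost pawn that glides in a straight line from a screen-space direction, locked until an actor overlap resets its movement mode.
; Tick runs the mode-driven swept move, then capsule-traces ahead.
; A hit prints the actor and adds a half-speed slide along the surface; otherwise the mode move runs again.
; Bounce reflection is disconnected and SlidingMovement is an unused stub.
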(event `self.ReceiveActorBeginOverlap`
  (params (OtherActor :type "Actor Object Reference"))
  (set `self.CurrentMovementMode` "NewEnumerator0"))

(event `self.ReceiveTick`
  (params (DeltaSeconds :type "Float (single-precision)"))
  (bind _returnvalue (`self.K2_GetActorLocation`))
  (`self.MovementFunc_Tick`)
  (bind (_outhit _returnvalue_2) (`KismetSystemLibrary.CapsuleTraceSingleForObjects` :`Start` _returnvalue :`End` (+ _returnvalue (* (`self.Direction`) (`self.Speed`) (`GameplayStatics.GetWorldDeltaSeconds`))) :`Radius` 40.0 :`HalfHeight` 50.0 :`ObjectTypes` (`self.Object Types`) :`DrawTime` 10.0))
  (if _returnvalue_2
    (bind (_bblockinghit _binitialoverlap _time _distance _location _impactpoint _normal _impactnormal _physmat _hitactor) (`GameplayStatics.BreakHitResult` _outhit))
    (`KismetSystemLibrary.PrintString` (`KismetSystemLibrary.GetDisplayName` _hitactor) true true (struct :`G` 0.66 :`B` 1.0 :`A` 1.0) 5.0)
    (`self.K2_AddActorWorldOffset` (* (`KismetMathLibrary.Normal` (- (`self.Direction`) (* (`KismetMathLibrary.Dot_VectorVector` (`self.Direction`) _impactnormal) _impactnormal))) (`self.Speed`) (`GameplayStatics.GetWorldDeltaSeconds`) (0.5 0.5 0.5)) true)
    (else
      (`self.MovementFunc_Tick`))))

(event `wdebr4te`
  (params (ScreenDir :type "Vector2D Structure"))
  (bind (_x _y) (`KismetMathLibrary.BreakVector2D` ScreenDir))
  (if (`|EnumInequality` (`self.CurrentMovementMode`) "NewEnumerator1")
    (set `self.Direction` (`KismetMathLibrary.MakeVector` _y (* _x -1.0)))
    (set `self.CurrentMovementMode` "NewEnumerator1")))

(fn `GligingMovement`
  (returns (SweepHitResult :type "HitResult Structure"))
  (bind _sweephitresult (`self.K2_AddActorWorldOffset` (* (`self.Direction`) (`self.Speed`) (`GameplayStatics.GetWorldDeltaSeconds`)) true))
  (return _sweephitresult))

(fn `MovementFunc_Tick`
  (switch `/Game/Root/Blueprints/Character/BE_GhostMovement` (`self.CurrentMovementMode`)
    (:`NewEnumerator1`
      (bind _sweephitresult (`self.GligingMovement`)))))

(fn `SlidingMovement`
  (bind (_outhit _returnvalue) (`KismetSystemLibrary.CapsuleTraceSingleForObjects` (`self.K2_GetActorLocation`) (0.0 0.0 0.0) 0.0 0.0 (`self.Object Types`)))
  (if _returnvalue
    _))

(fn `UserConstructionScript`)