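; Player controller that turns left mouse clicks into a 2D direction for the player's ghost pawn.
; On BeginPlay it shows the mouse cursor and caches the possessed B_GhostPawn.
; Each click projects the pawn's location to screen space, subtracts the cursor position and normalizes the result.
; That vector, pointing from cursor toward pawn, is passed to the pawn's Wdebr4te function.
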(event `self.ReceiveBeginPlay`
  (set `self.bShowMouseCursor` true)
  (bind _asb_ghost_pawn (cast `/Game/Root/Blueprints/Character/B_GhostPawn` (`GameplayStatics.GetPlayerPawn` 0)))
  (set `self.GhostPawn` _asb_ghost_pawn))

(event `Key|LeftMouseButton`
  (params (Key :type "Key Structure"))
  (bind (_locationx _locationy) (`self.GetMousePosition`))
  (:`Pressed`
    (`/Game/Root/Blueprints/Character/B_GhostPawn.wdebr4te` (`self.GhostPawn`) (`KismetMathLibrary.Normal2D` (- (`GameplayStatics.ProjectWorldToScreen` self (`self.K2_GetActorLocation` (`GameplayStatics.GetPlayerPawn` 0)) true) (`KismetMathLibrary.MakeVector2D` _locationx _locationy))))))

(fn `UserConstructionScript`)