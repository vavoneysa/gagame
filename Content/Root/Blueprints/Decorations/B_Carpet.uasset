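; Carpet decoration that slows B_GhostPawn and plays a dragging-feet sound while it moves over the carpet.
; Begin overlap on Carpet_Collision lowers the pawn's FloatingPawnMovement max speed and spawns a 2D sound through a DoOnce.
; End overlap raises the speed again and stops the sound.
; The DoOnce reset branch is unreachable because InCarpet is set true beforehand, so the sound spawns only on first entry.
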(event `self.Carpet_Collision.OnComponentBeginOverlap`
  (params (OverlappedComponent :type "PrimitiveComponent Object Reference") (OtherActor :type "Actor Object Reference") (OtherComp :type "PrimitiveComponent Object Reference") (OtherBodyIndex :type Integer) (bFromSweep :type Boolean) (SweepResult :type "HitResult Structure (by ref)"))
  (set `self.InCarpet` true)
  (bind _asb_ghost_pawn (cast `/Game/Root/Blueprints/Character/B_GhostPawn` OtherActor))
  (set `FloatingPawnMovement.MaxSpeed` 200.0 (`/Game/Root/Blueprints/Character/B_GhostPawn.FloatingPawnMovement` _asb_ghost_pawn))
  (if (`self.InCarpet`)
    (`/Engine/EditorBlueprintResources/StandardMacros.DoOnce` false :!label _label
      (:`Completed`
        (bind _returnvalue (`GameplayStatics.SpawnSound2D` "/Game/Root/Blueprints/Sounds/feet-drag-on-carpet-82522.feet-drag-on-carpet-82522" 1.0 1.0 0.0 null))))
    (else
      (goto _label :!via `Reset`))))

(event `self.Carpet_Collision.OnComponentEndOverlap`
  (params (OverlappedComponent :type "PrimitiveComponent Object Reference") (OtherActor :type "Actor Object Reference") (OtherComp :type "PrimitiveComponent Object Reference") (OtherBodyIndex :type Integer))
  (set `self.InCarpet` false)
  (bind _asb_ghost_pawn (cast `/Game/Root/Blueprints/Character/B_GhostPawn` OtherActor))
  (set `FloatingPawnMovement.MaxSpeed` 800.0 (`/Game/Root/Blueprints/Character/B_GhostPawn.FloatingPawnMovement` _asb_ghost_pawn))
  (`/Engine/EditorBlueprintResources/StandardMacros.IsValid` (stale `self.Carpet_Collision.OnComponentBeginOverlap` _returnvalue)
    (:`Is Valid`
      (`AudioComponent.Stop` (stale `self.Carpet_Collision.OnComponentBeginOverlap` _returnvalue)))))

(event `self.ReceiveActorBeginOverlap`
  (params (OtherActor :type "Actor Object Reference")))

(fn `UserConstructionScript`)