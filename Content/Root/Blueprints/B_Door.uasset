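; Door Blueprint that swings open when a B_GhostPawn enters its trigger box, then removes itself.
; It stores the door component's world rotation at BeginPlay as the closed position.
; The box overlap plays a timeline that lerps the door's yaw from that rotation by OpenAngle.
; A few seconds after the timeline finishes, the door component is destroyed, so it never closes again.
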(event `self.ReceiveBeginPlay`
  (set `self.ClosedPosition` (`SceneComponent.K2_GetComponentRotation` (`self.Door`))))

(event `self.Box.OnComponentBeginOverlap`
  (params (OverlappedComponent :type "PrimitiveComponent Object Reference") (OtherActor :type "Actor Object Reference") (OtherComp :type "PrimitiveComponent Object Reference") (OtherBodyIndex :type Integer) (bFromSweep :type Boolean) (SweepResult :type "HitResult Structure (by ref)"))
  (bind (_closedposition_roll _closedposition_pitch _closedposition_yaw) (`KismetMathLibrary.BreakRotator` (`self.ClosedPosition`)))
  (bind _door (`self.Door`))
  (cast `/Game/Root/Blueprints/Character/B_GhostPawn` OtherActor)
  (bind (_direction _open) (`Timeline|TL_DoorOpen`)
    (:`Update`
      (`SceneComponent.K2_SetWorldRotation` _door (`KismetMathLibrary.RLerp` (`self.ClosedPosition`) (`KismetMathLibrary.MakeRotator` _closedposition_roll _closedposition_pitch (+ (`self.Open Angle`) _closedposition_yaw)) _open) false false))
    (:`Finished`
      (`KismetSystemLibrary.Delay` 3.5)
      (`ActorComponent.K2_DestroyComponent` _door))))

(fn `UserConstructionScript`)