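; Behavior tree task that prepares patrol movement for BP_AIEnemy by picking a destination.
; It sets the enemy's walk speed to PatrolSpeed, then writes a random reachable point within Radius of the pawn to the PatrolLocation blackboard key, falling back to the pawn's own location.
; It finishes successfully at once without moving the pawn; leftover spline-following logic is disconnected and never runs.
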(event `self.ReceiveExecuteAI`
  (params (OwnerController :type "AIController Object Reference") (ControlledPawn :type "Pawn Object Reference"))
  (bind _returnvalue (`Actor.K2_GetActorLocation` ControlledPawn))
  (bind _patrollocation (`self.PatrolLocation`))
  (bind (_randomlocation _returnvalue_2) (`NavigationSystemV1.K2_GetRandomReachablePointInRadius` _returnvalue (`self.Radius`) null null))
  (bind _asbp_aienemy (cast `/Game/Root/Blueprints/Character/BP_AIEnemy` ControlledPawn))
  (set `CharacterMovementComponent.MaxWalkSpeed` (`self.PatrolSpeed`) (`Character.CharacterMovement` _asbp_aienemy))
  (if _returnvalue_2
    (`BTFunctionLibrary.SetBlackboardValueAsVector` _patrollocation _randomlocation)
    (else
      (`BTFunctionLibrary.SetBlackboardValueAsVector` _patrollocation _returnvalue)))
  (`self.FinishExecute` true))

(fn `NewFunction`)